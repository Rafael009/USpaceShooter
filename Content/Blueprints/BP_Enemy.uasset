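; BP_Enemy is an enemy actor that descends along Z and awards score when shot.
; Each Tick lowers it by Speed per frame, without delta-time scaling, then DestroyEnemy removes it once it reaches a lower Z limit.
; A sphere overlap with a BP_Shoot adds points through the GS_JogoPontuacao game state, then destroys both projectile and enemy.
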(event OnComponentBeginOverlap(Sphere)
  (params (OverlappedComponent :type Primitive%20Component%20Object%20Reference) (OtherActor :type Actor%20Object%20Reference) (OtherComp :type Primitive%20Component%20Object%20Reference) (OtherBodyIndex :type Integer) (bFromSweep :type Boolean) (SweepResult :type Hit%20Result%20Structure%20%28by%20ref%29))
  ;[1 1 1] Ponto e Destroy
  (bind _asbp_shoot (Utilities|Casting|CastToBP_Shoot OtherActor))
  (bind _asgs_jogo_pontuacao (Utilities|Casting|CastToGS_JogoPontuacao (Game|GetGameState)))
  (Default|AddScore _asgs_jogo_pontuacao 1e+01)
  (Actor|DestroyActor _asbp_shoot)
  (Actor|DestroyActor))

(event EventBeginPlay
  ;[1 1 1] Movimento
)

(event Collision|EventActorBeginOverlap
  (params (OtherActor :type Actor%20Object%20Reference)))

(event EventTick
  (params (DeltaSeconds :type Float%20%28single-precision%29))
  (bind _returnvalue (Transformation|GetActorLocation))
  ;[1 1 1] Movimento
  (Transformation|SetActorLocation (Math|Vector|MakeVector (.x _returnvalue) (.y _returnvalue) (- (.z _returnvalue) (Variables|Default|Getspeed))) false false)
  (CallFunction|DestroyEnemy -6e+02))

(fn ConstructionScript)

(fn DestroyEnemy
  (params (ZValue :type Float%20%28single-precision%29))
  (if (<= (.z (Transformation|GetActorLocation)) ZValue)
    (Actor|DestroyActor)))