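; GS_JogoPontuacao is a Blueprint that stores the game's score and life count, apparently as a GameState.
; Its construction script initializes Score to zero and Life to three through the setter functions.
; AddScore, SetScore and SetLife update and return their values, while DecLifes subtracts one life with no lower bound and always returns zero.
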(event EventBeginPlay)

(event EventTick
  (params (DeltaSeconds :type Float%20%28single-precision%29)))

(fn ConstructionScript
  (CallFunction|SetScore 0.0)
  (CallFunction|SetLife 3))

(fn AddScore
  (params (Valor :type Float%20%28single-precision%29))
  (bind _output_get (Variables|Default|SetScore (+ Valor (Variables|Default|GetScore))))
  (return _output_get))

(fn SetScore
  (params (Value :type Float%20%28single-precision%29))
  (bind _output_get (Variables|Default|SetScore Value))
  (return _output_get))

(fn SetLife
  (params (Value :type Integer))
  (bind _output_get (Variables|Default|SetLife Value))
  (return _output_get))

(fn DecLifes
  (Variables|Default|SetLife (- (Variables|Default|GetLife) 1))
  (return 0))